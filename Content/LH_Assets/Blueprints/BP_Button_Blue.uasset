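; Blue button actor that latches as pressed when Character1 or Character2 overlaps its box, signalling the blue level event.
; The box overlap tries both character casts and sets a pressed flag, which this Blueprint never clears.
; Tick polls that flag through a short Delay and, once set, repeatedly writes the event state to BlueEvent on GameMode_Game.
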(event `self.ReceiveTick`
  (params (DeltaSeconds :type "Float (single-precision)"))
  (`|ExecutionSequence`
    (:`then_0`
      (`KismetSystemLibrary.Delay` 0.1)
      (if (`self.HasBeenPresed`)
        (set `self.LevelEvent` true)
        (bind _asgame_mode_game (cast `/Game/GameMode_Game` (`GameplayStatics.GetGameMode`)))
        (set `/Game/GameMode_Game.Blue Event` (`self.LevelEvent`) _asgame_mode_game)))))

(event `self.Box.OnComponentBeginOverlap`
  (params (OverlappedComponent :type "PrimitiveComponent Object Reference") (OtherActor :type "Actor Object Reference") (OtherComp :type "PrimitiveComponent Object Reference") (OtherBodyIndex :type Integer) (bFromSweep :type Boolean) (SweepResult :type "HitResult Structure (by ref)"))
  (`|ExecutionSequence`
    (:`then_0`
      (cast `/Game/LH_Assets/Blueprints/Character1` OtherActor)
      (set `self.HasBeenPresed` true))
    (:`then_1`
      (cast `/Game/LH_Assets/Blueprints/Character2` OtherActor)
      (set `self.HasBeenPresed` true))))

(fn `UserConstructionScript`)