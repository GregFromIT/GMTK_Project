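; Wall_10m is a movable level piece that slides a bridge mesh along a spline when a Blue or Yellow game event is active.
; The construction script assigns the mesh and places it at the spline start.
; Tick polls GameMode_Game through a 0.2-second Delay, with IsBlueEvent selecting the flag.
; Timelines drive position along the spline; Blue calls PlayFromStart on every passing poll, while Yellow calls Play.
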(event `self.ReceiveBeginPlay`
  (bind _asgame_mode_game (cast `/Game/GameMode_Game` (`GameplayStatics.GetGameMode`)))
  (set `self.gameMode` _asgame_mode_game))

(event `self.ReceiveTick`
  (params (DeltaSeconds :type "Float (single-precision)"))
  (bind _spline (`self.Spline`))
  (bind _spline_2 (`self.Spline`))
  (`|ExecutionSequence`
    (:`then_0`
      (`KismetSystemLibrary.Delay` 0.2)
      (if (`self.IsBlueEvent`)
        (if (`/Game/GameMode_Game.Blue Event` (`self.gameMode`))
          (bind (_direction _newtrack_0) (`Timeline|Timeline_0` :!via `PlayFromStart`)
            (:`Update`
              (`SceneComponent.K2_SetWorldLocation` (`self.Brige`) (`SplineComponent.GetLocationAtDistanceAlongSpline` _spline_2 (* _newtrack_0 (`SplineComponent.GetSplineLength` _spline_2)) "World") false false))))
        (elif (`/Game/GameMode_Game.Yellow Event` (`self.gameMode`))
          (bind (_direction_2 _newtrack_0_2) (`Timeline|Timeline_1`)
            (:`Update`
              (`SceneComponent.K2_SetWorldLocation` (`self.Brige`) (`SplineComponent.GetLocationAtDistanceAlongSpline` _spline (* _newtrack_0_2 (`SplineComponent.GetSplineLength` _spline)) "World") false false))))))))

(fn `UserConstructionScript`
  (`StaticMeshComponent.SetStaticMesh` (`self.Brige`) (`self.BridgeObj`))
  (`SceneComponent.K2_SetWorldLocation` (`self.Brige`) (`SplineComponent.GetLocationAtDistanceAlongSpline` (`self.Spline`) 0.0 "World") false false))