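; Yellow two-button actor that writes its LevelEvent value to YellowEvent on GameMode_Game.
; Two overlap boxes each set a pressed flag while Char_1 enters and clear it on exit.
; Tick, throttled by a short Delay, writes the event whenever the flags match, including when neither is pressed.
; The construction script places the two RedButton components at opposite ends of a spline.
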(event `self.ReceiveTick`
  (params (DeltaSeconds :type "Float (single-precision)"))
  (`|ExecutionSequence`
    (:`then_0`
      (`KismetSystemLibrary.Delay` 0.1)
      (if (== (`self.HasBeenPresed`) (`self.HasBeenPressed2`))
        (bind _asgame_mode_game (cast `/Game/GameMode_Game` (`GameplayStatics.GetGameMode`)))
        (set `/Game/GameMode_Game.YellowEvent` (`self.LevelEvent`) _asgame_mode_game)))))

(event `self.Box.OnComponentBeginOverlap`
  (params (OverlappedComponent :type "PrimitiveComponent Object Reference") (OtherActor :type "Actor Object Reference") (OtherComp :type "PrimitiveComponent Object Reference") (OtherBodyIndex :type Integer) (bFromSweep :type Boolean) (SweepResult :type "HitResult Structure (by ref)"))
  (`|ExecutionSequence`
    (:`then_0`
      (cast `/Game/SC_Assets/Char_1` OtherActor)
      (set `self.HasBeenPresed` true))
    (:`then_1`
      (cast `/Game/SC_Assets/Char_1` OtherActor)
      (set `self.HasBeenPresed` true))))

(event `self.Box1.OnComponentBeginOverlap`
  (params (OverlappedComponent :type "PrimitiveComponent Object Reference") (OtherActor :type "Actor Object Reference") (OtherComp :type "PrimitiveComponent Object Reference") (OtherBodyIndex :type Integer) (bFromSweep :type Boolean) (SweepResult :type "HitResult Structure (by ref)"))
  (`|ExecutionSequence`
    (:`then_0`
      (cast `/Game/SC_Assets/Char_1` OtherActor)
      (set `self.HasBeenPressed2` true))
    (:`then_1`
      (cast `/Game/SC_Assets/Char_1` OtherActor)
      (set `self.HasBeenPressed2` true))))

(event `self.Box.OnComponentEndOverlap`
  (params (OverlappedComponent :type "PrimitiveComponent Object Reference") (OtherActor :type "Actor Object Reference") (OtherComp :type "PrimitiveComponent Object Reference") (OtherBodyIndex :type Integer))
  (`|ExecutionSequence`
    (:`then_0`
      (cast `/Game/SC_Assets/Char_1` OtherActor)
      (set `self.HasBeenPresed` false))
    (:`then_1`
      (cast `/Game/SC_Assets/Char_1` OtherActor)
      (set `self.HasBeenPresed` false))))

(event `self.Box1.OnComponentEndOverlap`
  (params (OverlappedComponent :type "PrimitiveComponent Object Reference") (OtherActor :type "Actor Object Reference") (OtherComp :type "PrimitiveComponent Object Reference") (OtherBodyIndex :type Integer))
  (`|ExecutionSequence`
    (:`then_0`
      (cast `/Game/SC_Assets/Char_1` OtherActor)
      (set `self.HasBeenPressed2` false))
    (:`then_1`
      (cast `/Game/SC_Assets/Char_1` OtherActor)
      (set `self.HasBeenPressed2` false))))

(fn `UserConstructionScript`
  (bind _spline (`self.Spline`))
  (`SceneComponent.K2_SetWorldLocation` (`self.Red_Button_1`) (`SplineComponent.GetLocationAtDistanceAlongSpline` _spline 0.0 "World") false false)
  (`SceneComponent.K2_SetWorldLocation` (`self.Red_Button_2`) (`SplineComponent.GetLocationAtDistanceAlongSpline` _spline (`SplineComponent.GetSplineLength` _spline) "World") false false))