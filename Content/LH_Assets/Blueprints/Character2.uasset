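; Character2 is a second character apparently meant to mirror the player's Character1, which it caches on BeginPlay.
; Tick, after a short delay, prints a debug vector and enables walking only while the player moves horizontally, otherwise disabling movement.
; CopyMovement issues AI MoveTo toward a point built from player velocity and rotated location, negated when MovementDir is false.
; Its calls are disconnected, so that movement never runs here.
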(event `self.ReceiveBeginPlay`
  (`|ExecutionSequence`
    (:`then_0`
      (bind _asthird_person_character_1 (cast `/Game/LH_Assets/Blueprints/Character1` (`GameplayStatics.GetPlayerCharacter` 0)))
      (set `self.CharacterREF` _asthird_person_character_1))))

(event `CopyMovement`
  (bind _characterref (`self.CharacterREF`))
  (bind _returnvalue (`self.GetVelocity` _characterref))
  (bind _returnvalue_2 (`SceneComponent.K2_GetComponentLocation` (`Character.CapsuleComponent` _characterref)))
  (bind _returnvalue_3 (`KismetMathLibrary.MakeVector` (.x (/ (+ _returnvalue (`KismetMathLibrary.RotateAngleAxis` _returnvalue_2 90.0)) 2.0)) (.y (/ (+ _returnvalue (`KismetMathLibrary.RotateAngleAxis` _returnvalue_2 180.0)) 2.0))))
  (if (`self.MovementDir`)
    (`|AIMoveTo` self _returnvalue_3 null 1.0)
    (else
      (`|AIMoveTo` self (* _returnvalue_3 -1.0) null 0.0))))

(event `self.ReceiveTick`
  (params (DeltaSeconds :type "Float (single-precision)"))
  (bind _characterref (`self.CharacterREF`))
  (bind _charactermovement (`self.CharacterMovement`))
  (bind _returnvalue (`SceneComponent.K2_GetComponentLocation` (`Character.CapsuleComponent` (`self.CharacterREF`))))
  (`KismetSystemLibrary.Delay` 0.1)
  (`KismetSystemLibrary.PrintString` (`KismetStringLibrary.Conv_VectorToString` (* (`KismetMathLibrary.MakeVector` (.x (/ (+ (`self.GetVelocity` _characterref) (`KismetMathLibrary.RotateAngleAxis` _returnvalue 270.0)) 2.0)) (.y (`KismetMathLibrary.RotateAngleAxis` _returnvalue 180.0 (0.0 1.0 0.0)))) -1.0)))
  (if (not (or (!= (.x (`self.GetVelocity` _characterref)) 0.0) (!= (.y (`self.GetVelocity` _characterref)) 0.0)))
    (`CharacterMovementComponent.SetMovementMode` _charactermovement "MOVE_None" 0)
    (else
      (`CharacterMovementComponent.SetMovementMode` _charactermovement "MOVE_Walking" 0))))

(fn `UserConstructionScript`)